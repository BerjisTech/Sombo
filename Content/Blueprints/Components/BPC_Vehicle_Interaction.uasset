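; Vehicle component for Bp_vehicle_base_pawn that handles engine audio, speed boost and driver exit.
; StartEngine adds an attenuated engine sound, and Tick maps engine rotation speed to its RPMRange parameter.
; Boost input adds current velocity plus the forward vector onto the player vehicle's velocity, roughly doubling it.
; Interact input detaches and repossesses the Driver at the exit point, then destroys the engine audio; BrakeLights is an empty stub.
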(event `self.ReceiveBeginPlay`
  (`self.setUpVehicle`))

(event `StartEngine`
  (`self.addEngine`))

(event `self.ReceiveTick`
  (params (DeltaSeconds :type "Float (single-precision)"))
  (`self.adjustEngineSound`))

(event `EnhancedInput|/Sombo/Blueprints/Input/IA_Speed_Boost`
  (params (ActionValue :type Boolean) (ElapsedSeconds :type "Float (double-precision)") (TriggeredSeconds :type "Float (double-precision)") (InputAction :type "InputAction Object Reference" :default "/Sombo/Blueprints/Input/IA_Speed_Boost.IA_Speed_Boost"))
  (:`Started`
    (`self.Boost Vehicle Speed`)))

(event `Boost Vehicle Speed`
  (bind _returnvalue (`GameplayStatics.GetPlayerPawn` 0))
  (bind _mesh (`WheeledVehiclePawn.Mesh` (cast `WheeledVehiclePawn` _returnvalue :!pure true)))
  (if (`GameplayStatics.ObjectIsA` _returnvalue "/Sombo/Blueprints/Vehicles/Blueprints/bp_vehicle_base_pawn.bp_vehicle_base_pawn_C")
    (bind _returnvalue_2 (`PrimitiveComponent.GetPhysicsLinearVelocity` _mesh "None"))
    (`PrimitiveComponent.SetPhysicsLinearVelocity` _mesh (+ _returnvalue_2 (`SceneComponent.GetForwardVector` _mesh)) true "None")))

(event `EnhancedInput|/Sombo/Blueprints/Input/IA_Interact`
  (params (ActionValue :type Boolean) (ElapsedSeconds :type "Float (double-precision)") (TriggeredSeconds :type "Float (double-precision)") (InputAction :type "InputAction Object Reference" :default "/Sombo/Blueprints/Input/IA_Interact.IA_Interact"))
  (:`Started`
    (`self.Unposses Vehicle`)))

(event `Unposses Vehicle`
  (bind _returnvalue (`self.GetOwner`))
  (bind _driver (`self.Driver`))
  (bind _asbp_vehicle_base_pawn (cast `/Sombo/Blueprints/Vehicles/Blueprints/bp_vehicle_base_pawn` _returnvalue)
    (:`then`
      (bind _driver_2 (`self.Driver`)
        (:`then`
          (`Actor.K2_DetachFromActor` _driver_2 "KeepWorld" "KeepWorld" "KeepWorld")
          (`Controller.Possess` (`GameplayStatics.GetPlayerController` 0) _driver_2)
          (`Actor.SetActorEnableCollision` _driver true)
          (`Actor.K2_SetActorTransform` _driver (`SceneComponent.K2_GetComponentToWorld` (`/Sombo/Blueprints/Vehicles/Blueprints/bp_vehicle_base_pawn.DriverExitPoint` _asbp_vehicle_base_pawn)) false true)
          (set `self.has_driver` false)
          (set `self.Driver` null)
          (`self.removeEngine`))
        (:`else`)))
    (:`CastFailed`
      (`KismetSystemLibrary.PrintString` (`KismetStringLibrary.Concat_StrStr` "Couldn't cast " (`KismetSystemLibrary.GetDisplayName` _returnvalue) " to vehicle base pawn") true true (struct :`G` 0.66 :`B` 1.0 :`A` 1.0) 10.0))))

(fn `BrakeLights`
  (params (BrakeLights :type Boolean)))