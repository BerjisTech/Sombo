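; Radio component that plays songs from a list of stations as 2D sound, with a widget for the radio.
; Each song's finished event starts the next, looping within the station, while playNext unbinds it, stops playback and cycles to the next station's first song.
; IA_Radio creates the widget on Triggered and removes it on Completed or Canceled.
; Up and Down keys step the volume multiplier.
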(event `playRadio`
  (bind _output_get (set `self.currentRadio` (`|GetArrayItem` (`self.radios`) (`self.currentRadioIndex`))))
  (bind _output_get_2 (set `self.currentSong` (`|GetArrayItem` (`.songs_7_E82B70B44158FC183254BCACFC08D5A9` (break `/Sombo/Blueprints/PlayerData/Struct_RadioSongs` _output_get)) (`self.currentSongIndex`))))
  (bind _returnvalue (`GameplayStatics.CreateSound2D` _output_get_2 1.0 1.0 0.0 null false false))
  (bind _output_get_3 (set `self.sound2d` _returnvalue))
  (add `AudioComponent.OnAudioFinished` _output_get_3 (delegate `OnAudioFinished_Event`))
  (`AudioComponent.Play` _output_get_3 0.0))

(event `OnAudioFinished_Event`
  (bind _currentsongindex (`self.currentSongIndex`))
  (bind (_currentradio_radio _currentradio_songs) (break `/Sombo/Blueprints/PlayerData/Struct_RadioSongs` (`self.currentRadio`)))
  (set `self.currentSongIndex` (`KismetMathLibrary.SelectInt` 0 (+ _currentsongindex 1) (== _currentsongindex (`KismetArrayLibrary.Array_LastIndex` _currentradio_songs))))
  (`self.playRadio`))

(event `Key|R`
  (params (Key :type "Key Structure")))

(event `playNext`
  (bind _currentradioindex (`self.currentRadioIndex`))
  (bind _sound2d (`self.sound2d`))
  (`/Engine/EditorBlueprintResources/StandardMacros.IsValid` _sound2d
    (:`Is Valid`
      (set `self.currentRadioIndex` (`KismetMathLibrary.SelectInt` 0 (+ _currentradioindex 1) (== _currentradioindex (`KismetArrayLibrary.Array_LastIndex` (`self.radios`)))))
      (set `self.currentSongIndex` 0)
      (clear `AudioComponent.OnAudioFinished` _sound2d)
      (`AudioComponent.Stop` _sound2d))
    (:`Is Not Valid`
      _))
  (`self.playRadio`))

(event `EnhancedInput|/Sombo/Blueprints/Input/IA_Radio`
  (params (ActionValue :type Boolean) (ElapsedSeconds :type "Float (double-precision)") (TriggeredSeconds :type "Float (double-precision)") (InputAction :type "InputAction Object Reference" :default "/Sombo/Blueprints/Input/IA_Radio.IA_Radio"))
  (:`Triggered`
    (`self.create radio widget`))
  (:`Canceled`
    (`self.destroy radio widget` :!label _label))
  (:`Completed`
    (goto _label)))

(event `Key|Down`
  (params (Key :type "Key Structure"))
  (bind _sound2d (`self.sound2d`))
  (:`Pressed`
    (`AudioComponent.SetVolumeMultiplier` _sound2d (- (`AudioComponent.VolumeMultiplier` _sound2d) 0.1))))

(event `Key|Up`
  (params (Key :type "Key Structure"))
  (bind _sound2d (`self.sound2d`))
  (:`Pressed`
    (`AudioComponent.SetVolumeMultiplier` _sound2d (+ (`AudioComponent.VolumeMultiplier` _sound2d) 0.1))))