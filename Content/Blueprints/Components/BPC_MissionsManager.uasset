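; Player character component that runs missions, currently a timed "Arrival" objective to reach a destination.
; On BeginPlay it caches sibling components such as UI and SaveLoad, then picks the mission from the saved active mission.
; Arrival sets the HUD brief and spawns a landscape-aligned marker at an offset from the player.
; A looping Delay polls distance each second, feeds the countdown pointer, and reports pass or fail through a temporary alert widget.
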(event `self.ReceiveBeginPlay`
  (`self.setPlayerData`)
  (`self.chooseMission`))

(event `self.ReceiveTick`
  (params (DeltaSeconds :type "Float (single-precision)")))