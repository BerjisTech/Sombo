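; Debug component with test helpers for teleporting the player and previewing money-change notifications.
; The IA_Teleport input moves the player character to a random PlayerStart.
; UpdateMoneyBalance reuses the parent's first WBP_Money child or adds a new one, fills it with fake text, and removes it after five seconds.
; The fake-update helper builds rich text with a random amount and independently random sign and success/danger style.
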(event `self.ReceiveBeginPlay`)

(event `EnhancedInput|/Sombo/Blueprints/Input/IA_Teleport`
  (params (ActionValue :type Boolean) (ElapsedSeconds :type "Float (double-precision)") (TriggeredSeconds :type "Float (double-precision)") (InputAction :type "InputAction Object Reference" :default "/Sombo/Blueprints/Input/IA_Teleport.IA_Teleport"))
  (:`Triggered`
    (bind _outactors (`GameplayStatics.GetAllActorsOfClass` "/Script/Engine.PlayerStart"))
    (`Actor.K2_SetActorTransform` (`GameplayStatics.GetPlayerCharacter` 0) (`Actor.GetTransform` (`KismetArrayLibrary.Array_Random` _outactors)) false true)))