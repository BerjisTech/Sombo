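; Save/load component that persists player progress (location, stats, money, missions, owned assets) in a GS_PlayerProgress save slot.
; BeginPlay loads or creates the save, applying stored movement stats and location on load, then autosaves on a repeating 0.2-second delay.
; A load/unload widget macro wraps both operations in loading screens.
; A ragdoll, kill-cam and random-PlayerStart respawn handler exists, but its damage binding and HUD updates are disconnected.
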(event `self.ReceiveBeginPlay`
  (`self.FindGameSave`)
  (`self.Save Game`))

(event `self.ReceiveTick`
  (params (DeltaSeconds :type "Float (single-precision)"))
  (`self.Handle Player Damage`))

(event `Handle Player Damage`)

(event `FindGameSave`
  (bind _returnvalue (`GameplayStatics.DoesSaveGameExist` (`self.DefaultSlot`)))
  (if _returnvalue
    (`self.LoadGameSave`)
    (else
      (`self.CreateGameSave`))))

(event `OnTakeAnyDamage_Event`
  (params (DamagedActor :type "Actor Object Reference") (Damage :type "Float (single-precision)") (DamageType :type "DamageType Object Reference") (InstigatedBy :type "Controller Object Reference") (DamageCauser :type "Actor Object Reference"))
  (bind _returnvalue (`GameplayStatics.GetPlayerCharacter` 0))
  (bind _stats_maxhealth (break `/Sombo/Blueprints/PlayerData/Struct_Stats` (`/Sombo/Blueprints/PlayerData/GS_PlayerProgress.Stats` (`self.ActiveGame`))))
  (bind _mesh (`Character.Mesh` _returnvalue))
  (bind _capsulecomponent (`Character.CapsuleComponent` _returnvalue))
  (bind _output_get (set `self.Current Health` (- (`self.Current Health`) Damage)))
  (if (< _output_get 1.0)
    (bind _foundwidgets (`WidgetBlueprintLibrary.GetAllWidgetsOfClass` "/Sombo/Blueprints/UI/WBP_KillCam.WBP_KillCam_C"))
    (if (`KismetArrayLibrary.Array_IsEmpty` _foundwidgets)
      (`PrimitiveComponent.SetSimulatePhysics` (`Character.Mesh` (`GameplayStatics.GetPlayerCharacter` 0)) true)
      (`KismetSystemLibrary.Delay` 1.0)
      (bind _returnvalue_2 (`|CreateWidget` "/Sombo/Blueprints/UI/WBP_KillCam.WBP_KillCam_C" (`GameplayStatics.GetPlayerController` 0)))
      (`UserWidget.AddToViewport` _returnvalue_2 0)
      (bind _outactors (`GameplayStatics.GetAllActorsOfClass` "/Script/Engine.PlayerStart"))
      (`KismetSystemLibrary.Delay` 2.0)
      (`Actor.K2_SetActorTransform` _returnvalue (`Actor.GetTransform` (`KismetArrayLibrary.Array_Random` _outactors)) false true)
      (`SceneComponent.K2_AttachToComponent` _mesh _capsulecomponent "None" "KeepRelative" "KeepRelative" "KeepRelative" true)
      (`SceneComponent.K2_SetRelativeLocationAndRotation` _mesh (`KismetMathLibrary.MakeVector` 0.0 0.0 (* (.z (`.BoxExtent` (`KismetSystemLibrary.GetComponentBounds` _capsulecomponent))) -1.0)) (struct :`Yaw` -90.0) false true)
      (`PrimitiveComponent.SetSimulatePhysics` _mesh false)
      (set `self.Current Health` _stats_maxhealth)
      (`KismetSystemLibrary.Delay` 3.0)
      (bind _foundwidgets_2 (`WidgetBlueprintLibrary.GetAllWidgetsOfClass` "/Sombo/Blueprints/UI/WBP_KillCam.WBP_KillCam_C"))
      (for _array_element _foundwidgets_2
        (`Widget.RemoveFromParent` _array_element)))))

(event `LoadGameSave`
  (`self.Load Unload Widget` "/Sombo/Blueprints/UI/WBP_LoadingScreen.WBP_LoadingScreen_C" :!label _label
    (:`Loaded`
      (bind _returnvalue (`GameplayStatics.LoadGameFromSlot` (`self.DefaultSlot`)))
      (`/Engine/EditorBlueprintResources/StandardMacros.IsValid` _returnvalue
        (:`Is Valid`
          (set `self.ActiveGame` (cast `/Sombo/Blueprints/PlayerData/GS_PlayerProgress` _returnvalue :!pure true))
          (goto _label :!via `Unload`))))
    (:`Unloaded`
      (`self.Save Local Variables`)
      (`self.UpdatePlayerDetails`))))

(event `CreateGameSave`
  (bind _returnvalue (`GameplayStatics.CreateSaveGameObject` "/Sombo/Blueprints/PlayerData/GS_PlayerProgress.GS_PlayerProgress_C"))
  (set `self.ActiveGame` _returnvalue))

(event `Save Game`
  (`self.Save Game Variables` :!label _label_2)
  (`KismetSystemLibrary.Delay` 0.2)
  (goto _label_2))