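; Garage actor that parks the player's driven vehicle and opens the garage UI when it enters a trigger box.
; If free, it teleports and stops the vehicle at a parking point; with an interaction component, it flags it in-garage, shows WBP_GarageUI with UI-only input, switches the camera and marks itself occupied.
; If occupied, it sends the vehicle back outside.
; Ending overlap closes the UI, restores game input and camera, and frees the garage.
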(event `self.Box.OnComponentBeginOverlap`
  (params (OverlappedComponent :type "PrimitiveComponent Object Reference") (OtherActor :type "Actor Object Reference") (OtherComp :type "PrimitiveComponent Object Reference") (OtherBodyIndex :type Integer) (bFromSweep :type Boolean) (SweepResult :type "HitResult Structure (by ref)"))
  (bind _returnvalue (`GameplayStatics.GetPlayerController` 0))
  (bind _asbp_vehicle_base_pawn (cast `/Sombo/Blueprints/Vehicles/Blueprints/bp_vehicle_base_pawn` OtherActor :!pure true))
  (bind _returnvalue_2 (`self.GetComponentByClass` _asbp_vehicle_base_pawn "/Sombo/Blueprints/Components/BPC_Vehicle_Interaction.BPC_Vehicle_Interaction_C"))
  (if (and (`GameplayStatics.ObjectIsA` OtherActor "/Sombo/Blueprints/Vehicles/Blueprints/bp_vehicle_base_pawn.bp_vehicle_base_pawn_C") (== OtherActor (`Controller.K2_GetPawn` (`GameplayStatics.GetPlayerController` 0))))
    (if (`self.occupied`)
      (`self.sendBack` OtherActor)
      (else
        (`self.K2_SetActorTransform` OtherActor (`SceneComponent.K2_GetComponentToWorld` (`self.VehicleParking`)) false true)
        (`/Sombo/Blueprints/Vehicles/Blueprints/bp_vehicle_base_pawn.DeadStop` _asbp_vehicle_base_pawn)
        (`/Engine/EditorBlueprintResources/StandardMacros.IsValid` _returnvalue_2
          (:`Is Valid`
            (set `/Sombo/Blueprints/Components/BPC_Vehicle_Interaction.is_in_garage` true _returnvalue_2)
            (bind _returnvalue_3 (`|CreateWidget` "/Sombo/Blueprints/UI/WBP_GarageUI.WBP_GarageUI_C" (`GameplayStatics.GetPlayerController` 0)))
            (`UserWidget.AddToViewport` _returnvalue_3 0)
            (`WidgetBlueprintLibrary.SetInputMode_UIOnlyEx` _returnvalue _returnvalue_3)
            (set `/Sombo/Blueprints/UI/WBP_GarageUI.vehicleInGarage` _asbp_vehicle_base_pawn _returnvalue_3)
            (set `PlayerController.bShowMouseCursor` true _returnvalue)
            (`PrimitiveComponent.SetPhysicsLinearVelocity` (`WheeledVehiclePawn.Mesh` _asbp_vehicle_base_pawn) (0.0 0.0 0.0) true "None")
            (`SceneComponent.K2_SetRelativeTransform` (`/Sombo/Blueprints/Vehicles/Blueprints/bp_vehicle_base_pawn.BackSpringArm` _asbp_vehicle_base_pawn) (`SceneComponent.GetRelativeTransform` (`/Sombo/Blueprints/Vehicles/Blueprints/bp_vehicle_base_pawn.bodyCamera` _asbp_vehicle_base_pawn)) false true)
            (set `self.occupied` true)))))))

(event `self.Box.OnComponentEndOverlap`
  (params (OverlappedComponent :type "PrimitiveComponent Object Reference") (OtherActor :type "Actor Object Reference") (OtherComp :type "PrimitiveComponent Object Reference") (OtherBodyIndex :type Integer))
  (bind _returnvalue (`GameplayStatics.GetPlayerController` 0))
  (bind _foundwidgets (`WidgetBlueprintLibrary.GetAllWidgetsOfClass` "/Sombo/Blueprints/UI/WBP_GarageUI.WBP_GarageUI_C"))
  (for _array_element _foundwidgets
    (`Widget.RemoveFromParent` _array_element)
    (`WidgetBlueprintLibrary.SetInputMode_GameOnly` _returnvalue true)
    (set `PlayerController.bShowMouseCursor` false _returnvalue)
    (bind _vehicleingarage (`/Sombo/Blueprints/UI/WBP_GarageUI.vehicleInGarage` _array_element))
    (`SceneComponent.K2_SetRelativeTransform` (`/Sombo/Blueprints/Vehicles/Blueprints/bp_vehicle_base_pawn.BackSpringArm` _vehicleingarage) (`SceneComponent.GetRelativeTransform` (`/Sombo/Blueprints/Vehicles/Blueprints/bp_vehicle_base_pawn.defaultBackCamera` _vehicleingarage)) false true)
    (set `self.occupied` false)))

(fn `UserConstructionScript`)