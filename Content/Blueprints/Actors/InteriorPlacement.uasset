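; InteriorPlacement is an actor that brings up the interior placement UI and handles a spawn request.
; On BeginPlay it removes any existing top-level WBP_InteriorPlacement widgets, then creates a fresh one and initializes it with a reference to itself.
; Its Spawner event destroys every BP_P_Furniture actor in the level, then spawns a BP_MissionMarker at the supplied location.
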(event `self.ReceiveBeginPlay`
  (bind _foundwidgets (`WidgetBlueprintLibrary.GetAllWidgetsOfClass` "/Sombo/Blueprints/UI/WBP_InteriorPlacement.WBP_InteriorPlacement_C"))
  (for _array_element _foundwidgets
    (`Widget.RemoveFromParent` _array_element))
  (bind _returnvalue (`|CreateWidget` "/Sombo/Blueprints/UI/WBP_InteriorPlacement.WBP_InteriorPlacement_C"))
  (`UserWidget.AddToViewport` _returnvalue 0)
  (`/Sombo/Blueprints/UI/WBP_InteriorPlacement.Initialize` _returnvalue self))

(event `Spawner`
  (params (`Spawn Transform Location` :type "Vector Structure"))
  (bind _outactors (`GameplayStatics.GetAllActorsOfClass` "/Sombo/BrutalistLevelKit/Blueprints/Furniture/Parent/BP_P_Furniture.BP_P_Furniture_C"))
  (for _array_element _outactors
    (`self.K2_DestroyActor` _array_element))
  (`|SpawnActorFromClass` "/Sombo/Blueprints/Actors/BP_MissionMarker.BP_MissionMarker_C" (`KismetMathLibrary.MakeTransform` `Spawn Transform Location`) "Undefined" "MultiplyWithRoot" null null))

(fn `UserConstructionScript`)