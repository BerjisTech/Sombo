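; Winged vehicle Blueprint that translates player input into aircraft-style control on its vehicle movement component.
; Look input drives pitch and roll on every trigger state, scaled by a fixed multiplier.
; Steering input switches by movement state, acting as ground steering when the component is moving on the ground and as yaw otherwise.
; BeginPlay extends the parent setup by clearing the grounded flag and setting a long spring arm for the camera.
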(event `self.ReceiveBeginPlay`
  (`parent.ReceiveBeginPlay`)
  (set `self.is_grounded` false)
  (set `self.Spring Arm Length` 4000.0))

(event `self.ReceiveTick`
  (params (DeltaSeconds :type "Float (single-precision)"))
  (`parent.ReceiveTick` DeltaSeconds))

(event `EnhancedInput|/Sombo/Blueprints/Input/IA_Look`
  (params (ActionValue :type "Vector2D Structure") (ElapsedSeconds :type "Float (double-precision)") (TriggeredSeconds :type "Float (double-precision)") (InputAction :type "InputAction Object Reference" :default "/Sombo/Blueprints/Input/IA_Look.IA_Look"))
  (bind _vehiclemovementcomponent (`self.VehicleMovementComponent`))
  (:`Triggered`
    (`ChaosVehicleMovementComponent.SetPitchInput` _vehiclemovementcomponent (* ActionValue_Y 250.0) :!label _label)
    (`ChaosVehicleMovementComponent.SetRollInput` _vehiclemovementcomponent (* ActionValue_X 250.0)))
  (:`Started`
    (goto _label))
  (:`Ongoing`
    (goto _label))
  (:`Canceled`
    (goto _label))
  (:`Completed`
    (goto _label)))

(event `EnhancedInput|/Sombo/Blueprints/Input/IA_Steering`
  (params (ActionValue :type "Float (double-precision)") (ElapsedSeconds :type "Float (double-precision)") (TriggeredSeconds :type "Float (double-precision)") (InputAction :type "InputAction Object Reference" :default "/Sombo/Blueprints/Input/IA_Steering.IA_Steering"))
  (bind _returnvalue (* ActionValue 250.0))
  (bind _vehiclemovementcomponent (`self.VehicleMovementComponent`))
  (:`Triggered`
    (if (`NavMovementComponent.IsMovingOnGround` _vehiclemovementcomponent) :!label _label_2
      (`ChaosVehicleMovementComponent.SetSteeringInput` _vehiclemovementcomponent _returnvalue)
      (else
        (`ChaosVehicleMovementComponent.SetYawInput` _vehiclemovementcomponent _returnvalue))))
  (:`Completed`
    (goto _label_2)))

(fn `UserConstructionScript`
  (`parent.UserConstructionScript`))